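; BP_LabIllumination is a lab light actor that blinks on and off at irregular intervals while changing colour.
; Tick runs through a Delay that acts as a repeating timer, toggling GenLight's visibility and rerolling the wait to a random few seconds.
; An incrementing counter modulo three sets the colour on each toggle, red on every third step and green otherwise, including toggles that switch the light off.
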(event `self.ReceiveTick`
  (params (DeltaSeconds :type "Float (single-precision)"))
  (bind _genlight (`self.GenLight`))
  (`KismetSystemLibrary.Delay` (`self.Espera`))
  (`SceneComponent.SetVisibility` _genlight (not (`SceneComponent.bVisible` _genlight)) false)
  (set `self.Espera` (`KismetMathLibrary.RandomFloatInRange` 2.2 7.7))
  (bind _result (`/Engine/EditorBlueprintResources/StandardMacros.IncrementInt` (`self.Color`))
    (:`  `
      (bind _output_get (set `self.Color` _result))
      (if (`KismetMathLibrary.Conv_IntToBool` (mod _output_get 3))
        (`LightComponent.SetLightColor` _genlight (make `LinearColor` 0.0 1.0 0.24) true)
        (else
          (`LightComponent.SetLightColor` _genlight (make `LinearColor` 1.0 0.0 0.03) true))))))

(fn `UserConstructionScript`)
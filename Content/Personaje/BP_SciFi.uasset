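; BP_SciFi is an actor whose PointLight switches on when the player's ThirdPersonCharacter touches its Sphere.
; Sphere overlap and hit events both cast to the character and make the light visible, and nothing here turns it off.
; Disconnected leftover chains would also increment the character's coin count, update its coin widget and, in one case, play a sound, but they never run.
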(event `self.Sphere.OnComponentBeginOverlap`
  (params (OverlappedComponent :type "PrimitiveComponent Object Reference") (OtherActor :type "Actor Object Reference") (OtherComp :type "PrimitiveComponent Object Reference") (OtherBodyIndex :type Integer) (bFromSweep :type Boolean) (SweepResult :type "HitResult Structure (by ref)"))
  (bind _pointlight (`self.PointLight`))
  (cast `/Game/ThirdPersonBP/Blueprints/ThirdPersonCharacter_` OtherActor)
  (if (not (`SceneComponent.bVisible` _pointlight))
    (`SceneComponent.SetVisibility` _pointlight true false)))

(event `self.Sphere.OnComponentHit`
  (params (HitComponent :type "PrimitiveComponent Object Reference") (OtherActor :type "Actor Object Reference") (OtherComp :type "PrimitiveComponent Object Reference") (NormalImpulse :type "Vector Structure") (Hit :type "HitResult Structure (by ref)"))
  (cast `/Game/ThirdPersonBP/Blueprints/ThirdPersonCharacter_` OtherActor)
  (`SceneComponent.SetVisibility` (`self.PointLight`) true false))

(fn `UserConstructionScript`)